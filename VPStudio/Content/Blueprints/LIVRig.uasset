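; LIV camera rig Blueprint that turns pasted LIV pose text into measured joint offsets.
; SetConfig parses key=value entries into a map, taking rx/ry as tilt and pan and scaling x/y/z from Unity to Unreal units.
; Those assignments and the following UpdateJoints call run only when the PrintMapValues debug flag is on.
; The construction script also calls UpdateJoints, which is defined outside this graph.
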(fn `GenerateMapFromString`
  (params (Input :type String))
  (returns (Map :type "Map of String to Float (double-precision)"))
  (locals (GenMap :type "Map of String to Float (double-precision)"))
  (bind _genmap (`local.GenMap`))
  ;[1 1 1] Convert the strings into a map
  (for _array_element (`KismetStringLibrary.ParseIntoArray` Input " \n")
    (bind (_lefts _rights _returnvalue) (`KismetStringLibrary.Split` _array_element "="))
    (if _returnvalue
      (`BlueprintMapLibrary.Map_Add` _genmap _lefts (`KismetStringLibrary.Conv_StringToDouble` _rights))
      (set `self.PoseMap` _genmap)))
  (return (`local.GenMap`)))

(fn `PrintMapValues`
  (params (`Input Map` :type "Map of String to Float (double-precision)") (`Print to Screen` :type Boolean) (`Print to Log` :type Boolean))
  ;[1 1 1] Print out map contents
  (`|ExecutionSequence`
    (:`then_0`
      (bind _values (`BlueprintMapLibrary.Map_Values` `Input Map`))
      (for _array_element _values
        (`KismetSystemLibrary.PrintString` (`KismetStringLibrary.Conv_DoubleToString` _array_element) `Print to Screen` `Print to Log` (struct :`R` 1.0 :`B` 0.672742 :`A` 1.0))))
    (:`then_1`
      (bind _keys (`BlueprintMapLibrary.Map_Keys` `Input Map`))
      (for _array_element_2 _keys
        (`KismetSystemLibrary.PrintString` _array_element_2 `Print to Screen` `Print to Log` (struct :`G` 1.0 :`B` 0.013699 :`A` 1.0))
        (return)))))

(fn `SetConfig`
  (bind _liv_pose_text (`self.LIV Pose Text`))
  (bind _unitytounrealmultiplier (`self.UnityToUnrealMultiplier`))
  (bind _posemap (`self.PoseMap`))
  (if (> (`KismetStringLibrary.Len` _liv_pose_text) 0)
    (bind _map (`self.GenerateMapFromString` _liv_pose_text))
    (bind _output_get (set `self.PoseMap` _map))
    (if (`self.Print Map Values`)
      (`self.PrintMapValues` _output_get true true)
      (`|ExecutionSequence`
        (:`then_0`
          ;[1 1 1] Set Rotation offset
          (set `self.Measured Pan` (`BlueprintMapLibrary.Map_Find` _posemap "ry")))
        (:`then_1`
          (set `self.Measured Tilt` (`BlueprintMapLibrary.Map_Find` _posemap "rx")))
        (:`then_2`
          ;[1 1 1] Set Position offset
          (set `self.Measured Horizontal` (* 1 (* _unitytounrealmultiplier (`BlueprintMapLibrary.Map_Find` _posemap "x")))))
        (:`then_3`
          (set `self.Measured EntrancePupil` (* 1 (* _unitytounrealmultiplier (`BlueprintMapLibrary.Map_Find` _posemap "z")))))
        (:`then_4`
          (set `self.Measured Vertical` (* 1 (* _unitytounrealmultiplier (`BlueprintMapLibrary.Map_Find` _posemap "y")))))
        (:`then_5`
          (`self.Update Joints`))))
    (else
      (`KismetSystemLibrary.PrintString` "Please enter LIV data into correct field before proceeding." true true (struct :`R` 1.0 :`A` 1.0) 4.0))))

(fn `UserConstructionScript`
  (`self.Update Joints`))